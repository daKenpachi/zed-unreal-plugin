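; BP_ZEDCamera is a ZED camera Blueprint that manages scene captures and image planes for combining video with virtual content.
; Two seconds after BeginPlay, or on request, it copies FOV and custom projection settings from the left intermediate capture to the left virtual capture.
; Events apply a non-empty hidden-actor list to both intermediate captures.
; Others hide the intermediate and final planes from the left virtual capture, or clear its hidden components.
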(event `SetSceneCaptureSettings`
  (bind _virtualleftcamera (`self.VirtualLeftCamera`))
  (bind _interleftcamera (`self.InterLeftCamera`))
  (set `SceneCaptureComponent2D.FOVAngle` (`SceneCaptureComponent2D.FOVAngle` _interleftcamera) _virtualleftcamera :!label _label)
  (set `SceneCaptureComponent2D.bUseCustomProjectionMatrix` (`SceneCaptureComponent2D.bUseCustomProjectionMatrix` _interleftcamera) _virtualleftcamera)
  (set `SceneCaptureComponent2D.CustomProjectionMatrix` (`SceneCaptureComponent2D.CustomProjectionMatrix` _interleftcamera) _virtualleftcamera))

(event `HideActorsInVideo`
  (bind _hiddenactors (`self.HiddenActors`))
  (if (> (`KismetArrayLibrary.Array_Length` _hiddenactors) 0)
    (set `SceneCaptureComponent.HiddenActors` _hiddenactors (`self.InterLeftCamera`))
    (set `SceneCaptureComponent.HiddenActors` _hiddenactors (`self.InterRightCamera`))))

(event `self.ReceiveBeginPlay`
  (`KismetSystemLibrary.Delay` 2.0)
  (goto _label))

(event `HideCameraPlanes`
  (bind _virtualleftcamera (`self.VirtualLeftCamera`))
  (`SceneCaptureComponent.HideComponent` _virtualleftcamera (`self.FinalLeftPlane`))
  (`SceneCaptureComponent.HideComponent` _virtualleftcamera (`self.FinalRightPlane`))
  (`SceneCaptureComponent.HideComponent` _virtualleftcamera (`self.InterLeftPlane`))
  (`SceneCaptureComponent.HideComponent` _virtualleftcamera (`self.InterRightPlane`)))

(event `ShowCameraPlanes`
  (`SceneCaptureComponent.ClearHiddenComponents` (`self.VirtualLeftCamera`)))

(fn `UserConstructionScript`)