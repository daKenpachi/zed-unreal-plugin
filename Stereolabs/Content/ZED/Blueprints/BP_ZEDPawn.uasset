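; ZED pawn Blueprint that shows temporary log messages through a stereo layer.
; The construction script assigns a log render target to the layer, and BeginPlay draws a material onto it, then clears it.
; PrintOnLog draws colored text onto that target and starts a timer for the given duration.
; The timer calls ClearLog, which draws a reset texture over the target and invalidates the timer.
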(event `self.ReceiveBeginPlay`
  (bind (_canvas _size _context) (`KismetRenderingLibrary.BeginDrawCanvasToRenderTarget` (`self.LogRenderTarget`)))
  (`Canvas.K2_DrawMaterial` _canvas "/Game/UI/LogRenderMaterial.LogRenderMaterial" (0.0 0.0) _size (0.0 0.0) (1.0 1.0) 0.0 (0.5 0.5))
  (`KismetRenderingLibrary.EndDrawCanvasToRenderTarget` _context)
  (`self.ClearLog`))

(event `ClearLog`
  (bind (_canvas _size _context) (`KismetRenderingLibrary.BeginDrawCanvasToRenderTarget` (`self.LogRenderTarget`)))
  (`Canvas.K2_DrawTexture` _canvas "/Game/UI/ResetLogRenderTarget.ResetLogRenderTarget" (0.0 0.0) _size (0.0 0.0) (1.0 1.0) (struct :`R` 1.0 :`G` 1.0 :`B` 1.0 :`A` 1.0) "BLEND_Translucent" 0.0 (0.5 0.5))
  (`KismetRenderingLibrary.EndDrawCanvasToRenderTarget` _context)
  (if (`KismetSystemLibrary.K2_IsValidTimerHandle` (stale `PrintOnLog` _returnvalue))
    (`KismetSystemLibrary.K2_ClearAndInvalidateTimerHandle` (stale `PrintOnLog` _returnvalue))))

(event `PrintOnLog`
  (params (String :type String :default "Hello LOG") (Color :type "LinearColor Structure" :default (struct :`R` 1.0 :`G` 1.0 :`B` 1.0 :`A` 1.0)) (Duration :type "Float (double-precision)" :default 5.0))
  (bind (_canvas _size _context) (`KismetRenderingLibrary.BeginDrawCanvasToRenderTarget` (`self.LogRenderTarget`)))
  (`Canvas.K2_DrawText` _canvas "/Game/UI/LogFont.LogFont" String (10.0 10.0) Color 0.0 (struct :`A` 1.0) (1.0 1.0) false false false (struct :`A` 1.0))
  (`KismetRenderingLibrary.EndDrawCanvasToRenderTarget` _context)
  (bind _returnvalue (`KismetSystemLibrary.K2_SetTimerDelegate` (delegate `ClearLog`) Duration)))

(fn `UserConstructionScript`
  (`StereoLayerComponent.SetTexture` (`self.StereoLayerLog`) (`self.LogRenderTarget`)))